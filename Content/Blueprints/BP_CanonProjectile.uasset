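; Cannon projectile actor that damages the player and lets them know when it is within interaction range.
; HitCollision destroys it on a blocking hit or on overlapping anything but itself or the player.
; Damage is dealt when the player's overlap with HitCollision ends, provided the Used flag is unset; this file never sets it.
; InteractionCollision passes overlap start and stop to the player through calls on the cached player reference.
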(event OnComponentEndOverlap(InteractionCollision)
  (params (OverlappedComponent :type Primitive%20Component%20Object%20Reference) (OtherActor :type Actor%20Object%20Reference) (OtherComp :type Primitive%20Component%20Object%20Reference) (OtherBodyIndex :type Integer))
  (if (== (Variables|Default|GetPlayer%20Ref) OtherActor)
    (Default|CallStopProjectileOverlap (Variables|Default|GetPlayer%20Ref))))

(event OnComponentBeginOverlap(HitCollision)
  (params (OverlappedComponent :type Primitive%20Component%20Object%20Reference) (OtherActor :type Actor%20Object%20Reference) (OtherComp :type Primitive%20Component%20Object%20Reference) (OtherBodyIndex :type Integer) (bFromSweep :type Boolean) (SweepResult :type Hit%20Result%20Structure%20%28by%20ref%29))
  (CallFunction|HitProcessing OtherActor))

(event OnComponentEndOverlap(HitCollision)
  (params (OverlappedComponent :type Primitive%20Component%20Object%20Reference) (OtherActor :type Actor%20Object%20Reference) (OtherComp :type Primitive%20Component%20Object%20Reference) (OtherBodyIndex :type Integer))
  (CallFunction|DamageValidation OtherActor))

(event OnComponentHit(HitCollision)
  (params (HitComponent :type Primitive%20Component%20Object%20Reference) (OtherActor :type Actor%20Object%20Reference) (OtherComp :type Primitive%20Component%20Object%20Reference) (NormalImpulse :type Vector :default "0, 0, 0") (Hit :type Hit%20Result%20Structure%20%28by%20ref%29))
  (Actor|DestroyActor))

(event OnComponentBeginOverlap(InteractionCollision)
  (params (OverlappedComponent :type Primitive%20Component%20Object%20Reference) (OtherActor :type Actor%20Object%20Reference) (OtherComp :type Primitive%20Component%20Object%20Reference) (OtherBodyIndex :type Integer) (bFromSweep :type Boolean) (SweepResult :type Hit%20Result%20Structure%20%28by%20ref%29))
  (if (== (Variables|Default|GetPlayer%20Ref) OtherActor)
    (Default|CallStartProjectileOverlap (Variables|Default|GetPlayer%20Ref) self)))

(event EventBeginPlay
  (bind _playerref (Class|BPIPlayer|GetPlayer(Message) (Game|GetPlayerCharacter 0)))
  (Variables|Default|SetPlayer%20Ref _playerref))

(fn ConstructionScript)

(fn HitProcessing
  (params (OtherActor :type Actor%20Object%20Reference))
  (if (!= OtherActor self)
    (bind _playerref (Class|BPIPlayer|GetPlayer(Message) (Game|GetPlayerCharacter 0)))
    (if (!= _playerref OtherActor)
      (Actor|DestroyActor))))

(fn DamageValidation
  (params (OtherActor :type Actor%20Object%20Reference))
  (bind _playerref (Class|BPIPlayer|GetPlayer(Message) (Game|GetPlayerCharacter 0)))
  (if (Math|Boolean|ANDBoolean (== _playerref OtherActor) (!= OtherActor self) (not (Variables|Default|GetbUsed)))
    (CallFunction|DealDamage self (Variables|Default|GetPlayer%20Ref) 1e+01)))