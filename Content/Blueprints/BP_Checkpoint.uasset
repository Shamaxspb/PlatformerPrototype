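; BP_Checkpoint is a checkpoint actor that registers itself as the player's LastCheckpoint when reached.
; An overlap on ReachTrigger calls SetNewCheckpoint, which identifies the player by checking that GetPlayerMessage on the overlapping actor returns that same actor.
; A successful check prints the checkpoint's name as reached.
; The trigger disables its collision after the first overlap, whether or not that actor is the player.
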(event OnComponentBeginOverlap(ReachTrigger)
  (params (OverlappedComponent :type Primitive%20Component%20Object%20Reference) (OtherActor :type Actor%20Object%20Reference) (OtherComp :type Primitive%20Component%20Object%20Reference) (OtherBodyIndex :type Integer) (bFromSweep :type Boolean) (SweepResult :type Hit%20Result%20Structure%20%28by%20ref%29))
  (CallFunction|SetNewCheckpoint OtherActor)
  (Collision|SetCollisionEnabled (Variables|Default|GetReachTrigger) "NoCollision"))

(fn ConstructionScript)

(fn SetNewCheckpoint
  (params (Other%20Actor :type Actor%20Object%20Reference))
  (bind _playerref (Class|BPIPlayer|GetPlayer(Message) Other%20Actor))
  (bind _output_get (Variables|Default|SetPlayer _playerref))
  (if (== _output_get Other%20Actor)
    (bind _output_get_2 (Variables|/Game/Blueprints/BP_Player.BP_Player_C|SetLastCheckpoint (Variables|Default|GetPlayer) self))
    (Development|PrintString (Utilities|String|Append (Utilities|GetDisplayName _output_get_2) " reached") true true "(R=0.273151,G=0.078125,B=1.000000,A=1.000000)")))