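; Spring actor that launches the player character when it hits the collision box.
; The hit event identifies the player through a GetPlayerMessage call, then applies LaunchCharacter with both XY and Z overrides.
; GetLaunchVector points opposite the impact normal at SpringPower magnitude and draws a debug arrow along it.
; The begin-overlap event only stores and checks the player, with no further action.
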(event OnComponentBeginOverlap(BoxCollision)
  (params (OverlappedComponent :type Primitive%20Component%20Object%20Reference) (OtherActor :type Actor%20Object%20Reference) (OtherComp :type Primitive%20Component%20Object%20Reference) (OtherBodyIndex :type Integer) (bFromSweep :type Boolean) (SweepResult :type Hit%20Result%20Structure%20%28by%20ref%29))
  (bind _playerref (Class|BPIPlayer|GetPlayer(Message) OtherActor))
  (bind _output_get (Variables|Default|SetPlayer _playerref))
  (if (== _output_get OtherActor)
    _))

(event OnComponentHit(BoxCollision)
  (params (HitComponent :type Primitive%20Component%20Object%20Reference) (OtherActor :type Actor%20Object%20Reference) (OtherComp :type Primitive%20Component%20Object%20Reference) (NormalImpulse :type Vector :default "0, 0, 0") (Hit :type Hit%20Result%20Structure%20%28by%20ref%29))
  (bind _playerref (Class|BPIPlayer|GetPlayer(Message) OtherActor))
  (bind _output_get (Variables|Default|SetPlayer _playerref))
  (if (== _output_get OtherActor)
    (Character|LaunchCharacter (Variables|Default|GetPlayer) (CallFunction|GetLaunchVector (.ImpactNormal (Collision|BreakHitResult Hit))) true true)))

(fn ConstructionScript)

(fn GetLaunchVector
  (params (Normal :type Vector))
  (bind _springpower (Variables|SpringConfig|GetSpringPower))
  (bind _boxcollision (Variables|Default|GetBoxCollision))
  (bind _returnvalue (Transformation|GetWorldLocation _boxcollision))
  (bind _returnvalue_2 (* Normal _springpower))
  (bind _returnvalue_3 (* _returnvalue_2 -1.0))
  (bind _returnvalue_4 (+ _returnvalue _returnvalue_3))
  (Rendering|Debug|DrawDebugArrow _returnvalue _returnvalue_4 5e+01 "(R=1.000000,G=0.000000,B=0.000000,A=1.000000)" 1e+01 5.0)
  (return (* (Math|Vector|GetUnitDirection(Vector) _returnvalue _returnvalue_4) (Variables|SpringConfig|GetSpringPower))))