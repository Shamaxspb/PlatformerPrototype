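; BP_Obstacle is an obstacle actor that moves back and forth between its starting location and an offset given by AdditiveVector.
; BeginPlay caches the start location, then a looping timer on MoveInterval flip-flops the MoveObstacleTL timeline between forward and reverse playback.
; Timeline updates set the location without sweep through VInterpTo, feeding the timeline's Alpha in as DeltaTime alongside InterpSpeed.
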(event Custom|MoveObstacle
  (bind _initial_location (Variables|Default|GetInitial%20Location))
  (Utilities|FlowControl|FlipFlop
    (:A
      (bind _alpha (Timeline|MoveObstacleTL PlayFromStart)
        (:Update
          (Transformation|SetActorLocation (Math|Interpolation|VInterpTo _initial_location (+ _initial_location (Variables|Obstacleconfig|GetAdditive%20Vector)) _alpha (Variables|Obstacleconfig|GetInterp%20Speed)) false false))))
    (:B
      (Timeline|MoveObstacleTL ReverseFromEnd))))

(event EventBeginPlay
  (CallFunction|Init)
  (Utilities|Time|SetTimerbyEvent (delegate Custom|MoveObstacle) (Variables|Obstacleconfig|GetMove%20Interval) true))

(fn ConstructionScript)

(fn Init
  (Variables|Default|SetInitial%20Location (Transformation|GetActorLocation))
  (Components|Timeline|SetPlayRate (Variables|Default|GetMoveObstacleTL) (/ 1.0 1.0)))